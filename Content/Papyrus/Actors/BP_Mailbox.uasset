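; BP_Mailbox is a mailbox actor that can accept a paper while it is open.
; SetOpen stores the state, rotates the mailbox mesh between open and closed poses, and turns every material slot red when open or green when closed.
; The construction script and BeginPlay both apply the current state.
; InsterPaper closes an open mailbox and returns true, or returns false if it is already closed.
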(event `SetStaticMeshMaterial`
  (params (StaticMeshComponent :type "StaticMeshComponent Object Reference") (Material :type "MaterialInterface Object Reference"))
  (`/Engine/EditorBlueprintResources/StandardMacros.IsValid` StaticMeshComponent
    (:`Is Valid`
      (for (_ _array_index) (`MeshComponent.GetMaterials` StaticMeshComponent)
        (`PrimitiveComponent.SetMaterial` StaticMeshComponent _array_index Material)))))

(event `SetOpen`
  (params (InOpen :type Boolean))
  (bind _output_get (set `self.Is Open` InOpen))
  (`|ExecutionSequence`
    (:`then_0`
      (`SceneComponent.K2_SetRelativeRotation` (`self.SM_Mailbox`) (`KismetMathLibrary.SelectRotator` (struct :`Roll` 90.0) (struct) _output_get) false false))
    (:`then_1`
      (bind _returnvalue (select `bool` _output_get :`false` "/Game/LevelPrototyping/Materials/MI_Solid_Green.MI_Solid_Green" :`true` "/Game/LevelPrototyping/Materials/MI_Solid_Red.MI_Solid_Red" :!type "MaterialInterface Object Reference"))
      (`self.SetStaticMeshMaterial` (`self.Root`) _returnvalue)
      (`self.SetStaticMeshMaterial` (`self.SM_Mailbox`) _returnvalue))))

(event `self.ReceiveBeginPlay`
  (`self.SetOpen` (`self.Is Open`)))

(fn `InsterPaper`
  (returns (bSuccess :type Boolean))
  (if (`self.Is Open`)
    (`self.SetOpen` false)
    (return true)
    (else
      (return false))))

(fn `UserConstructionScript`
  (`self.SetOpen` (`self.Is Open`)))