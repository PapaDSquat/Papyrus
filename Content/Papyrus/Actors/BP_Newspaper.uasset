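; BP_Newspaper is a newspaper actor that can be delivered into mailboxes.
; The construction script records its spawn transform, and Tick enables gravity on the mesh once the paper is at least a set distance from that point.
; On a hit it offers itself to a BP_Mailbox and destroys itself if accepted.
; Any hit that leaves the paper valid also enables gravity.
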(event `self.ReceiveTick`
  (params (DeltaSeconds :type "Float (single-precision)"))
  (`self.HandleGravityRelease` DeltaSeconds))

(event `self.ReceiveHit`
  (params (MyComp :type "PrimitiveComponent Object Reference") (Other :type "Actor Object Reference") (OtherComp :type "PrimitiveComponent Object Reference") (bSelfMoved :type Boolean) (HitLocation :type "Vector Structure") (HitNormal :type "Vector Structure") (NormalImpulse :type "Vector Structure") (Hit :type "HitResult Structure (by ref)"))
  (`|ExecutionSequence`
    (:`then_0`
      (bind _asbp_mailbox (cast `/Game/Papyrus/Actors/BP_Mailbox` Other))
      (bind _bsuccess (`/Game/Papyrus/Actors/BP_Mailbox.InsterPaper` _asbp_mailbox))
      (if _bsuccess
        (`self.K2_DestroyActor`)))
    (:`then_5`
      (`/Engine/EditorBlueprintResources/StandardMacros.IsValid` self
        (:`Is Valid`
          (`PrimitiveComponent.SetEnableGravity` (`self.StaticMesh`) true))))))

(event `HandleGravityRelease`
  (params (DeltaSeconds :type "Float (double-precision)"))
  (bind _spawntransform_location (`KismetMathLibrary.BreakTransform` (`self.SpawnTransform`)))
  (if (>= (`KismetMathLibrary.Vector_Distance` (`self.K2_GetActorLocation`) _spawntransform_location) (`self.DistanceToEnableGravity`))
    (`PrimitiveComponent.SetEnableGravity` (`self.StaticMesh`) true)))

(fn `UserConstructionScript`
  (set `self.SpawnTransform` (`self.GetTransform`)))